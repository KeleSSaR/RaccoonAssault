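; BP_Piedra is a rock (piedra) actor in the Raccoon character's folder that reacts to hits, apparently a distraction object that makes noise on landing.
; Hitting an actor tagged Enemy spawns a tiny-scaled Niagara effect, then destroys the rock after a short DoOnce-gated delay.
; Any other hit reports an AI noise event, prints a landed message and destroys the rock after a longer delay.
; An explosion emitter node is left unconnected.
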(event `self.Piedra.OnComponentHit`
  (params (HitComponent :type "PrimitiveComponent Object Reference") (OtherActor :type "Actor Object Reference") (OtherComp :type "PrimitiveComponent Object Reference") (NormalImpulse :type "Vector Structure") (Hit :type "HitResult Structure (by ref)"))
  (if (`self.ActorHasTag` OtherActor "Enemy")
    (`NiagaraFunctionLibrary.SpawnSystemAtLocation` (`self.NIagara`) (`SceneComponent.K2_GetComponentLocation` (`self.Piedra`)) (struct) (1e-06 1e-06 1e-06))
    (`/Engine/EditorBlueprintResources/StandardMacros.DoOnce` false
      (:`Completed`
        (`KismetSystemLibrary.Delay` 2.0)))
    (else
      (`AISense_Hearing.ReportNoiseEvent` (`self.K2_GetActorLocation`) 1.0 self 3000.0)
      (`KismetSystemLibrary.PrintString` "Landed")
      (`KismetSystemLibrary.Delay` 5.0)))
  (`self.K2_DestroyActor`))

(fn `UserConstructionScript`)