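; Pushable object actor that the raccoon player can push or pull while holding interact, with an overlap-driven prompt widget.
; Box overlap starts a looping timer checking input and the movable flag set by ActivarObjeto.
; CanPush uses a player line trace and an obstruction box trace along the rounded player forward direction.
; Timelines move the object with the movement-disabled player attached; releasing interact or leaving the box detaches them.
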(event `self.ReceiveBeginPlay`
  ;[1 1 1] Comment
  (bind _returnvalue (`GameplayStatics.GetActorOfClass` "/Game/Characters/Raccoon/Blueprints/BP_Raccoon.BP_Raccoon_C"))
  (set `self.PLayerCharacter` _returnvalue))

(event `/Game/Characters/Raccoon/Blueprints/BP_Interface.ActivarObjeto`
  (set `self.EsMovible` true))

(event `COmprobando si esta a rango`
  (bind _playercharacter (`self.PLayerCharacter`))
  ;[1 1 1] Comment
  (bind _returnvalue (`KismetSystemLibrary.K2_SetTimerDelegate` (delegate `COmprobando si esta a rango`) 0.01 true))
  (if (`self.TieneLaE`)
    (if (`self.EsMovible`)
      (set `self.DireccionEmpuje` (`KismetMathLibrary.MakeVector` (`KismetMathLibrary.Conv_IntToDouble` (`KismetMathLibrary.Round` (.x (`self.GetActorForwardVector` (stale `self.Box.OnComponentBeginOverlap` OtherActor))))) (`KismetMathLibrary.Conv_IntToDouble` (`KismetMathLibrary.Round` (.y (`self.GetActorForwardVector` (stale `self.Box.OnComponentBeginOverlap` OtherActor))))) (`KismetMathLibrary.Conv_IntToDouble` (`KismetMathLibrary.Round` (.z (`self.GetActorForwardVector` (stale `self.Box.OnComponentBeginOverlap` OtherActor)))))))
      (bind _canpush (`self.CanPush`))
      (if _canpush
        (`CharacterMovementComponent.DisableMovement` (`Character.CharacterMovement` (`GameplayStatics.GetPlayerCharacter` 0)))
        (`/Game/Characters/Raccoon/Blueprints/BP_Raccoon.Get prepare` (`self.PLayerCharacter`))
        (switch `int` (`self.SeleccionDeMOv`)
          (:`1`
            (`self.Push`)
            (`/Game/Characters/Raccoon/Blueprints/BP_Raccoon.get Pushing` _playercharacter))
          (:`2`
            (`self.TiraPatras`)
            (`/Game/Characters/Raccoon/Blueprints/BP_Raccoon.Get pulling` _playercharacter)))
        (`self.K2_AttachToActor` (`GameplayStatics.GetPlayerCharacter` 0) self "None" "KeepWorld" "KeepWorld" "KeepWorld" true)))
    (else
      (`/Game/Characters/Raccoon/Blueprints/BP_Raccoon.ni push ni ostias` (`self.PLayerCharacter`)))))

(event `self.Box.OnComponentBeginOverlap`
  (params (OverlappedComponent :type "PrimitiveComponent Object Reference") (OtherActor :type "Actor Object Reference") (OtherComp :type "PrimitiveComponent Object Reference") (OtherBodyIndex :type Integer) (bFromSweep :type Boolean) (SweepResult :type "HitResult Structure (by ref)"))
  ;[1 1 1] Comment
  (if (== (`GameplayStatics.GetPlayerCharacter` 0) OtherActor)
    (`self.COmprobando si esta a rango`)))

(event `Parar comprobacion`
  ;[1 1 1] Comment
  (`KismetSystemLibrary.K2_ClearAndInvalidateTimerHandle` (stale `COmprobando si esta a rango` _returnvalue)))

(event `self.Box.OnComponentEndOverlap`
  (params (OverlappedComponent :type "PrimitiveComponent Object Reference") (OtherActor :type "Actor Object Reference") (OtherComp :type "PrimitiveComponent Object Reference") (OtherBodyIndex :type Integer))
  ;[1 1 1] Comment
  (`self.Parar comprobacion`)
  (`self.StopPush`))

(event `Push`
  ;[1 1 1] Custom Event que realiza el empuje del obeto comprobando si esta o no pulsada la e para poder empujar
  (set `self.PosicionActual` (`self.K2_GetActorLocation`))
  (bind (_direction _posicion_) (`Timeline|Timeline`)
    (:`Update`
      (`self.K2_SetActorRelativeLocation` (+ (`self.PosicionActual`) (* _posicion_ (`self.DireccionEmpuje`) (`self.DistanciaDeEmpuje`)))))))

(event `StopPush`
  (bind _returnvalue (`GameplayStatics.GetPlayerCharacter` 0))
  ;[1 1 1] Custom event que su funcion es que el personaje se pueda volver a mover y que se desvincule del objeto
  (`CharacterMovementComponent.SetMovementMode` (`Character.CharacterMovement` _returnvalue) "MOVE_Walking" 0)
  (`self.K2_DetachFromActor` _returnvalue "KeepWorld" "KeepWorld" "KeepWorld")
  (set `self.EsMovible` false))

(event `EnhancedInput|/Game/ThirdPerson/Input/Actions/IA_Pull`
  (params (ActionValue :type Boolean) (ElapsedSeconds :type "Float (double-precision)") (TriggeredSeconds :type "Float (double-precision)") (InputAction :type "InputAction Object Reference" :default "/Game/ThirdPerson/Input/Actions/IA_Pull.IA_Pull"))
  ;[1 1 1] Comment
  (:`Ongoing`
    (set `self.SeleccionDeMOv` 2))
  (:`Canceled`
    (set `self.SeleccionDeMOv` 0 :!label _label))
  (:`Completed`
    (goto _label)))

(event `TiraPatras`
  ;[1 1 1] Comment
  (set `self.PosicionActual` (`self.K2_GetActorLocation`))
  (bind (_direction _posicion_) (`Timeline|Timeline_0`)
    (:`Update`
      (`self.K2_SetActorRelativeLocation` (+ (`self.PosicionActual`) (* _posicion_ (`self.DireccionEmpuje`) (`self.DistanciaDeEmpuje`)))))))

(event `EnhancedInput|/Game/ThirdPerson/Input/Actions/IA_Interactuar`
  (params (ActionValue :type Boolean) (ElapsedSeconds :type "Float (double-precision)") (TriggeredSeconds :type "Float (double-precision)") (InputAction :type "InputAction Object Reference" :default "/Game/ThirdPerson/Input/Actions/IA_Interactuar.IA_Interactuar"))
  ;[1 1 1] Input (hold and release) para poder interactuar con el objeto empujable y actualizando el boleano correspondiente para la comprobacion posterior
  (:`Ongoing`
    (set `self.TieneLaE` true))
  (:`Canceled`
    (set `self.TieneLaE` false :!label _label_2)
    (`self.StopPush`)
    (set `self.EsMovible` false))
  (:`Completed`
    (goto _label_2)))

(event `Restar`
  ;[1 1 1] Comment
  (set `self.DireccionEmpuje` (`KismetMathLibrary.MakeVector` (`KismetMathLibrary.Conv_IntToDouble` (`KismetMathLibrary.Round` (.x (`self.GetActorForwardVector`)))) (`KismetMathLibrary.Conv_IntToDouble` (`KismetMathLibrary.Round` (.y (`self.GetActorForwardVector`)))) (`KismetMathLibrary.Conv_IntToDouble` (`KismetMathLibrary.Round` (.z (`self.GetActorForwardVector`)))))))

(event `EnhancedInput|/Game/ThirdPerson/Input/Actions/IA_push`
  (params (ActionValue :type Boolean) (ElapsedSeconds :type "Float (double-precision)") (TriggeredSeconds :type "Float (double-precision)") (InputAction :type "InputAction Object Reference" :default "/Game/ThirdPerson/Input/Actions/IA_push.IA_push"))
  ;[1 1 1] Comment
  (:`Ongoing`
    (set `self.SeleccionDeMOv` 1))
  (:`Canceled`
    (set `self.SeleccionDeMOv` 0 :!label _label_3))
  (:`Completed`
    (goto _label_3)))

(event `self.widget interactuar.OnComponentBeginOverlap`
  (params (OverlappedComponent :type "PrimitiveComponent Object Reference") (OtherActor :type "Actor Object Reference") (OtherComp :type "PrimitiveComponent Object Reference") (OtherBodyIndex :type Integer) (bFromSweep :type Boolean) (SweepResult :type "HitResult Structure (by ref)"))
  (if (`self.ActorHasTag` OtherActor "Player")
    (`SceneComponent.SetVisibility` (`self.Widget`) true false)))

(event `self.widget interactuar.OnComponentEndOverlap`
  (params (OverlappedComponent :type "PrimitiveComponent Object Reference") (OtherActor :type "Actor Object Reference") (OtherComp :type "PrimitiveComponent Object Reference") (OtherBodyIndex :type Integer))
  (if (`self.ActorHasTag` OtherActor "Player")
    (`SceneComponent.SetVisibility` (`self.Widget`) false false)))

(fn `CanPush`
  (returns (CanPush :type Boolean))
  (bind _returnvalue (`GameplayStatics.GetPlayerCharacter` 0))
  (bind _returnvalue_2 (`self.K2_GetActorLocation`))
  (bind _returnvalue_3 (`self.K2_GetActorLocation`))
  (bind _cube (`self.Cube`))
  (bind _cube_2 (`self.Cube`))
  (bind _returnvalue_4 (`self.K2_GetActorLocation` _returnvalue))
  (bind _array (`|MakeArray` _returnvalue :!type "Actor Object Reference"))
  (bind (_returnvalue_origin _returnvalue_boxextent) (`KismetMathLibrary.BreakBoxSphereBounds` (`StaticMesh.GetBounds` (`StaticMeshComponent.StaticMesh` _cube_2))))
  (bind (_returnvalue_origin_2 _returnvalue_boxextent_2) (`KismetMathLibrary.BreakBoxSphereBounds` (`StaticMesh.GetBounds` (`StaticMeshComponent.StaticMesh` _cube))))
  (bind (_outhit _returnvalue_5) (`KismetSystemLibrary.LineTraceSingle` _returnvalue_4 (* _returnvalue_4 (`self.GetActorForwardVector` _returnvalue)) "TraceTypeQuery1" false _array "None" false))
  (if _returnvalue_5
    (switch `int` (`self.SeleccionDeMOv`)
      (:`1`
        (bind (_outhit_2 _returnvalue_6) (`KismetSystemLibrary.BoxTraceSingle` (+ _returnvalue_2 (0.0 0.0 0.0)) (+ _returnvalue_2 (* (`self.DireccionEmpuje`) (`self.DistanciaDeEmpuje`) (1.0 1.0 1.0)) (0.0 0.0 0.0)) (* _returnvalue_boxextent_2 (`SceneComponent.RelativeScale3D` _cube) (0.8 0.8 0.8)) (struct) "TraceTypeQuery1"))
        (return (not _returnvalue_6)))
      (:`2`
        (bind (_outhit_3 _returnvalue_7) (`KismetSystemLibrary.BoxTraceSingle` (+ _returnvalue_3 (0.0 0.0 0.0)) (+ _returnvalue_3 (* (`self.DireccionEmpuje`) (`self.DistanciaDeEmpuje`) (-3.0 -3.0 0.0)) (0.0 0.0 0.0)) (* _returnvalue_boxextent (`SceneComponent.RelativeScale3D` _cube_2) (0.8 0.8 0.8)) (struct) "TraceTypeQuery1" false _array))
        (return (not _returnvalue_7))))
    (else
      (return false))))

(fn `UserConstructionScript`)