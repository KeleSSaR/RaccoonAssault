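; Owl camera enemy (CamaraBuho) that sweeps by rotating around the yaw it is placed at.
; A timeline starts on BeginPlay and adds its value to that initial yaw on the capsule; Detenerrotacion stops it and ReanudarRotacion resumes it.
; The vision-range overlap event is empty.
; An unwired branch would open L_Tutorial_test_02 when the raccoon player's HaEntrado flag is set.
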(event `Reanudar Rotacion`
  (bind (_direction _rotacioncamara) (`Timeline|RotacionCamara` :!label _label)
    (:`Update`
      (`SceneComponent.K2_SetWorldRotation` (`self.CapsuleComponent`) (`KismetMathLibrary.MakeRotator` 0.0 0.0 (+ _rotacioncamara (`self.Return Value Z (Yaw)`))) false false))))

(event `self.ReceiveBeginPlay`
  (bind (_returnvalue_roll _returnvalue_pitch _returnvalue_yaw) (`KismetMathLibrary.BreakRotator` (`self.K2_GetActorRotation` self)))
  (set `self.Return Value Z (Yaw)` _returnvalue_yaw)
  (goto _label))

(event `Detener rotacion`
  (goto _label :!via `Stop`))

(event `self.rango_vision_roomba_01.OnComponentBeginOverlap`
  (params (OverlappedComponent :type "PrimitiveComponent Object Reference") (OtherActor :type "Actor Object Reference") (OtherComp :type "PrimitiveComponent Object Reference") (OtherBodyIndex :type Integer) (bFromSweep :type Boolean) (SweepResult :type "HitResult Structure (by ref)")))

(fn `UserConstructionScript`)