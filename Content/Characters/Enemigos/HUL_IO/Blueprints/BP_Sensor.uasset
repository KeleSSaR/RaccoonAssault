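; BP_Sensor is a HUL_IO enemy character Blueprint that animates its upper wheel component and exposes walk-speed control.
; On BeginPlay, the Walinkg event starts a timeline that lerps the wheel's relative rotation from its current value toward a near-full turn.
; A separate UpdateWalkSpeed function sets the CharacterMovement max walk speed, independently of the wheel animation.
; No sensing logic is present despite the name.
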(event `self.ReceiveBeginPlay`
  (`self.Walinkg`))

(event `Walinkg`
  (bind (_direction _newtrack_0) (`Timeline|Timeline` :!via `PlayFromStart`)
    (:`Update`
      (`SceneComponent.K2_SetRelativeRotation` (`self.HUL-IO_RUEDA_SUP_01`) (`KismetMathLibrary.RLerp` (`SceneComponent.RelativeRotation` (`self.HUL-IO_RUEDA_SUP_01`)) (struct :`Roll` 359.0) _newtrack_0) false false))))

(fn `UpdateWalkSpeed`
  (params (`Max Walk Speed` :type "Float (single-precision)"))
  (set `CharacterMovementComponent.MaxWalkSpeed` `Max Walk Speed` (`self.CharacterMovement`)))

(fn `UserConstructionScript`)