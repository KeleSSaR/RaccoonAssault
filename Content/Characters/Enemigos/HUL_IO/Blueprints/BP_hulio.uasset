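; HUL-IO enemy character that catches the player raccoon and ends the attempt by opening the tutorial test level.
; A looping timer checks velocity to set walking and focus flags on its Anim Blueprint and play or stop a Timeline that spins six wheel meshes.
; Mesh, capsule or box contact with the player, unless the raccoon's kill animation is active, freezes the enemy, disables player input and blends the camera to it before the level loads.
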(event `self.ReceiveBeginPlay`
  (bind _asbpa_hulio (cast `/Game/Characters/Enemigos/HUL_IO/Blueprints/BPA_HULIO` (`SkeletalMeshComponent.GetAnimInstance` (`self.Mesh`))))
  (set `self.As BPa Hulio` _asbpa_hulio)
  (bind _returnvalue (`GameplayStatics.GetActorOfClass` "/Game/Characters/Raccoon/Blueprints/BP_Raccoon.BP_Raccoon_C"))
  (set `self.BP_Raccoon` _returnvalue)
  (`self.Walinkg`)
  (bind _returnvalue_2 (`KismetSystemLibrary.K2_SetTimerDelegate` (delegate `TestWalk`) 0.1 true))
  (`self.TestWalk`))

(event `TestWalk`
  (bind _as_bpa_hulio (`self.As BPa Hulio`))
  (if (`self.pillado`)
    (`KismetSystemLibrary.K2_ClearAndInvalidateTimerHandle` (stale `self.ReceiveBeginPlay` _returnvalue_2))
    (set `/Game/Characters/Enemigos/HUL_IO/Blueprints/BPA_HULIO.isFocus` false (`self.As BPa Hulio`) :!label _label)
    (`self.stopFocus`)
    (`self.StopWalinkg`)
    (set `/Game/Characters/Enemigos/HUL_IO/Blueprints/BPA_HULIO.isWalking` false _as_bpa_hulio)
    (elif (!= (`self.GetVelocity`) (0.0 0.0 0.0))
      (`self.Walinkg`)
      (set `/Game/Characters/Enemigos/HUL_IO/Blueprints/BPA_HULIO.isWalking` true _as_bpa_hulio)
      (else
        (goto _label)))))

(event `Focus`
  (if (not (`self.pillado`))
    (set `/Game/Characters/Enemigos/HUL_IO/Blueprints/BPA_HULIO.isFocus` true (`self.As BPa Hulio`))))

(event `stopFocus`
  (if (`self.pillado`)
    (set `/Game/Characters/Enemigos/HUL_IO/Blueprints/BPA_HULIO.isFocus` false (`self.As BPa Hulio`))))

(event `asdad`)

(event `Walinkg`
  (bind _rueda1 (`self.RUEDA1`))
  (bind _rueda2 (`self.RUEDA2`))
  (bind _rueda3 (`self.RUEDA3`))
  (bind _rueda4 (`self.RUEDA4`))
  (bind _rueda5 (`self.RUEDA5`))
  (bind _rueda6 (`self.RUEDA6`))
  (if (`/Game/Characters/Raccoon/Blueprints/BP_Raccoon.AnimacionKill` (`self.BP_Raccoon`))
    (bind (_direction _newtrack_0) (`Timeline|Timeline_0` :!via `Stop` :!label _label_2)
      (:`Update`
        (`self.TestParaRuedas` (`SceneComponent.RelativeRotation` _rueda1) _newtrack_0 _rueda1)
        (`self.TestParaRuedas` (`SceneComponent.RelativeRotation` _rueda2) _newtrack_0 _rueda2)
        (`self.TestParaRuedas` (`SceneComponent.RelativeRotation` _rueda3) _newtrack_0 _rueda3)
        (`self.TestParaRuedas` (struct) _newtrack_0 _rueda4 (`SceneComponent.RelativeRotation` _rueda4))
        (`self.TestParaRuedas` (struct) _newtrack_0 _rueda5 (`SceneComponent.RelativeRotation` _rueda5))
        (`self.TestParaRuedas` (struct) _newtrack_0 _rueda6 (`SceneComponent.RelativeRotation` _rueda6))))
    (else
      (set `self.walking` true)
      (goto _label_2 :!via `PlayFromStart`))))

(event `StopWalinkg`
  (`self.stopFocus`)
  (if (`/Game/Characters/Raccoon/Blueprints/BP_Raccoon.AnimacionKill` (`self.BP_Raccoon`))
    (goto _label_2 :!via `Stop`)
    (else
      (set `self.walking` false)
      (goto _label_2 :!via `Stop`))))

(event `self.Mesh.OnComponentHit`
  (params (HitComponent :type "PrimitiveComponent Object Reference") (OtherActor :type "Actor Object Reference") (OtherComp :type "PrimitiveComponent Object Reference") (NormalImpulse :type "Vector Structure") (Hit :type "HitResult Structure (by ref)"))
  (if (`self.ActorHasTag` (stale `self.Box.OnComponentBeginOverlap` OtherActor) "Player") :!label _label_3
    (if (not (`/Game/Characters/Raccoon/Blueprints/BP_Raccoon.AnimacionKill` (`self.BP_Raccoon`)))
      (`self.DehaloQuieto`)
      (`self.AnimacionCamara`)
      (`self.StopWalinkg`)
      (`self.stopFocus`))))

(event `self.Box.OnComponentBeginOverlap`
  (params (OverlappedComponent :type "PrimitiveComponent Object Reference") (OtherActor :type "Actor Object Reference") (OtherComp :type "PrimitiveComponent Object Reference") (OtherBodyIndex :type Integer) (bFromSweep :type Boolean) (SweepResult :type "HitResult Structure (by ref)"))
  (goto _label_3))

(event `self.CapsuleComponent.OnComponentHit`
  (params (HitComponent :type "PrimitiveComponent Object Reference") (OtherActor :type "Actor Object Reference") (OtherComp :type "PrimitiveComponent Object Reference") (NormalImpulse :type "Vector Structure") (Hit :type "HitResult Structure (by ref)"))
  (goto _label_3))

(event `AnimacionCamara`
  (bind _returnvalue (`GameplayStatics.GetPlayerController` 0))
  (bind _returnvalue_2 (`GameplayStatics.GetPlayerController` 0))
  (`PlayerController.SetViewTargetWithBlend` _returnvalue self 2.0 "VTBlend_Linear" 0.0 false)
  (`self.DisableInput` (`self.BP_Raccoon`) _returnvalue)
  (set `PlayerController.bShowMouseCursor` false _returnvalue_2)
  (set `PlayerController.bEnableClickEvents` false _returnvalue_2)
  (`KismetSystemLibrary.Delay` 3.0)
  (`GameplayStatics.OpenLevel` "L_Tutorial_test_02"))

(event `DehaloQuieto`
  (bind _as_bpa_hulio (`self.As BPa Hulio`))
  (set `CharacterMovementComponent.MaxWalkSpeed` 0.0 (`self.CharacterMovement`))
  (set `/Game/Characters/Enemigos/HUL_IO/Blueprints/BPA_HULIO.isWalking` false _as_bpa_hulio)
  (set `/Game/Characters/Enemigos/HUL_IO/Blueprints/BPA_HULIO.isFocus` false _as_bpa_hulio)
  (set `self.pillado` true)
  (`self.stopFocus`)
  (`/Engine/EditorBlueprintResources/StandardMacros.DoOnce` false
    (:`Completed`
      (`self.AnimacionCamara`))))

(fn `TestParaRuedas`
  (params (ROT_der :type "Rotator Structure") (Alpha :type "Float (single-precision)") (mesh :type "MeshComponent Object Reference") (ROT_izq :type "Rotator Structure"))
  (returns (NewParam :type Boolean))
  (`SceneComponent.K2_SetRelativeRotation` mesh (`KismetMathLibrary.RLerp` ROT_der (struct :`Roll` 720.0) Alpha) false false)
  (return false))

(fn `UpdateWalkSpeed`
  (params (`Max Walk Speed` :type "Float (single-precision)"))
  (set `CharacterMovementComponent.MaxWalkSpeed` `Max Walk Speed` (`self.CharacterMovement`)))

(fn `UserConstructionScript`)