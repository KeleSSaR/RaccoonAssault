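; Roomba enemy pawn that wanders the NavMesh, chases the raccoon player and opens the tutorial level on contact.
; Wandering turns via timeline toward random reachable points, then uses AIMoveTo.
; DetectionZone overlap starts a delayed line trace whose result is unused, then a fast turn and timer-driven pursuit at higher speed until overlap ends.
; Player overlap on its Button or hits from "Piedra"-tagged actors temporarily stun it, disabling detection and kills.
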(event `self.ReceiveBeginPlay`
  (bind _returnvalue (`GameplayStatics.GetActorOfClass` "/Game/Characters/Raccoon/Blueprints/BP_Raccoon.BP_Raccoon_C"))
  (set `self.As BP Third Person Character` _returnvalue)
  (`self.MoveNPC`))

(event `MoveNPC`
  ;[1 1 1] Roomba Movement In NavMesh
  (if (not (or (`self.Stunned`) (`self.Following Player`)))
    ;;[1 1 1] Set Random Location In NavMesh
    (bind _output_get (set `self.Random Location` (`NavigationSystemV1.K2_GetRandomReachablePointInRadius` (`self.K2_GetActorLocation`) 1000.0 null null)))
    (bind (_direction _newtrack_0) (`Timeline|Rotation` :!via `PlayFromStart` :!label _label)
      (:`Update`
        (if (or (`self.Stunned`) (`self.Following Player`))
          (goto _label :!via `Stop`)
          (else
            (bind (_returnvalue_roll _returnvalue_pitch _returnvalue_yaw) (`KismetMathLibrary.BreakRotator` (`KismetMathLibrary.RLerp` (`self.K2_GetActorRotation`) (`KismetMathLibrary.FindLookAtRotation` (`self.K2_GetActorLocation`) _output_get) _newtrack_0 true)))
            ;;[1 1 1] Roomba Looking At Tarjet Location
            (`SceneComponent.K2_SetWorldRotation` (`self.DefaultSceneRoot`) (`KismetMathLibrary.MakeRotator` 0.0 0.0 _returnvalue_yaw) false false))))
      (:`Finished`
        (if (or (`self.Stunned`) (`self.Following Player`))
          (goto _label :!via `Stop`)
          (else
            ;;[1 1 1] Set Movement
            (`|AIMoveTo` self (`self.Random Location`) null
              (:`OnSuccess`
                _)
              (:`OnFail`
                (`KismetSystemLibrary.Delay` 0.1)))
            (`self.MoveNPC`)))))))

(event `self.Button.OnComponentBeginOverlap`
  (params (OverlappedComponent :type "PrimitiveComponent Object Reference") (OtherActor :type "Actor Object Reference") (OtherComp :type "PrimitiveComponent Object Reference") (OtherBodyIndex :type Integer) (bFromSweep :type Boolean) (SweepResult :type "HitResult Structure (by ref)"))
  (bind _floatingpawnmovement (`self.FloatingPawnMovement`))
  ;[1 1 1] Roomba's Stun
  (if (`self.Stunned`)
    _
    (elif (== OtherActor (`self.As BP Third Person Character`))
      (`GameplayStatics.SpawnEmitterAtLocation` "/Game/StarterContent/Particles/P_Explosion.P_Explosion" (`SceneComponent.K2_GetComponentLocation` (`self.StaticMesh`)))
      (set `self.Stunned` true)
      (`MovementComponent.StopMovementImmediately` _floatingpawnmovement)
      (`NavMovementComponent.StopActiveMovement` _floatingpawnmovement)
      (`SceneComponent.SetVisibility` (`self.DetectionZone`) false false)
      (`KismetSystemLibrary.Delay` 60.0) ; Stunned Time
      (`SceneComponent.SetVisibility` (`self.DetectionZone`) false false)
      (set `self.Stunned` false)
      (if (`self.Following Player`)
        (`self.FindPlayer`)
        (else
          (`self.MoveNPC`))))))

(event `self.StaticMesh.OnComponentHit`
  (params (HitComponent :type "PrimitiveComponent Object Reference") (OtherActor :type "Actor Object Reference") (OtherComp :type "PrimitiveComponent Object Reference") (NormalImpulse :type "Vector Structure") (Hit :type "HitResult Structure (by ref)"))
  (bind _floatingpawnmovement (`self.FloatingPawnMovement`))
  (if (`self.Stunned`)
    _
    (elif (`self.ActorHasTag` OtherActor "Piedra")
      (`/Engine/EditorBlueprintResources/StandardMacros.DoOnce` false :!label _label_2
        (:`Completed`
          (`GameplayStatics.SpawnEmitterAtLocation` "/Game/StarterContent/Particles/P_Explosion.P_Explosion" (`SceneComponent.K2_GetComponentLocation` (`self.StaticMesh`)))
          (set `self.Stunned` true)
          (`MovementComponent.StopMovementImmediately` _floatingpawnmovement)
          (`NavMovementComponent.StopActiveMovement` _floatingpawnmovement)
          (`SceneComponent.SetVisibility` (`self.DetectionZone`) false false)
          (`PrimitiveComponent.SetCollisionProfileName` (`self.StaticMesh`) "IgnoreonlyPawn" true)
          (`KismetSystemLibrary.Delay` 15.0) ; Stunned Time
          (`PrimitiveComponent.SetCollisionProfileName` (`self.StaticMesh`) "BlockAllDynamic" true)
          (`SceneComponent.SetVisibility` (`self.DetectionZone`) true false)
          (`self.reset do once`)
          (set `self.Stunned` false)
          (if (`self.Following Player`)
            (`self.FindPlayer`)
            (else
              (`self.MoveNPC`))))))))

(event `reset do once`
  (goto _label_2 :!via `Reset`))

(event `self.Shape.OnComponentBeginOverlap`
  (params (OverlappedComponent :type "PrimitiveComponent Object Reference") (OtherActor :type "Actor Object Reference") (OtherComp :type "PrimitiveComponent Object Reference") (OtherBodyIndex :type Integer) (bFromSweep :type Boolean) (SweepResult :type "HitResult Structure (by ref)"))
  ;[1 1 1] Player's Death
  (if (`self.Stunned`)
    _
    (elif (== OtherActor (`self.As BP Third Person Character`))
      (`GameplayStatics.OpenLevel` "L_Tutorial_test_02"))))

(event `self.DetectionZone.OnComponentBeginOverlap`
  (params (OverlappedComponent :type "PrimitiveComponent Object Reference") (OtherActor :type "Actor Object Reference") (OtherComp :type "PrimitiveComponent Object Reference") (OtherBodyIndex :type Integer) (bFromSweep :type Boolean) (SweepResult :type "HitResult Structure (by ref)"))
  ;[1 1 1] Player Detected?
  (if (`self.Stunned`)
    _
    (elif (== OtherActor (`self.As BP Third Person Character`))
      (`NavMovementComponent.StopActiveMovement` (`self.FloatingPawnMovement`))
      (set `self.Following Player` true)
      (`self.FindPlayer`))))

(event `self.DetectionZone.OnComponentEndOverlap`
  (params (OverlappedComponent :type "PrimitiveComponent Object Reference") (OtherActor :type "Actor Object Reference") (OtherComp :type "PrimitiveComponent Object Reference") (OtherBodyIndex :type Integer))
  ;[1 1 1] Stop Pursuing Player
  (if (== OtherActor (`self.As BP Third Person Character`))
    (set `FloatingPawnMovement.MaxSpeed` 200.0 (`self.FloatingPawnMovement`))
    (`KismetSystemLibrary.K2_ClearTimer` null "SendRaycast")
    (`KismetSystemLibrary.K2_ClearAndInvalidateTimerHandle` (stale `PursuePlayer` _returnvalue))
    (set `self.Following Player` false)
    (`NavMovementComponent.StopActiveMovement` (`self.FloatingPawnMovement`))
    (`self.MoveNPC`)))

(event `FindPlayer`
  ;[1 1 1] Can the Roomba directly see the player?
  (if (not (`self.Stunned`))
    (`KismetSystemLibrary.K2_SetTimer` null "SendRaycast" 0.2 true)))

(event `PursuePlayer`
  (bind (_returnvalue_x _returnvalue_y) (`KismetMathLibrary.BreakVector` (`self.K2_GetActorLocation` (`self.As BP Third Person Character`))))
  (bind (_returnvalue_x_2 _returnvalue_y_2 _returnvalue_z) (`KismetMathLibrary.BreakVector` (`SceneComponent.K2_GetComponentLocation` (`self.DefaultSceneRoot`))))
  (bind (_returnvalue_roll _returnvalue_pitch _returnvalue_yaw) (`KismetMathLibrary.BreakRotator` (`KismetMathLibrary.RLerp` (`self.K2_GetActorRotation`) (`KismetMathLibrary.FindLookAtRotation` (`self.K2_GetActorLocation`) (`self.K2_GetActorLocation` (`self.As BP Third Person Character`))) 1.0 true)))
  ;[1 1 1] Pursue player
  (bind _returnvalue (`KismetSystemLibrary.K2_SetTimerDelegate` (delegate `PursuePlayer`) 0.015 true))
  (if (`self.PlayerAlive`)
    (`SceneComponent.K2_SetWorldRotation` (`self.DefaultSceneRoot`) (`KismetMathLibrary.MakeRotator` 0.0 0.0 _returnvalue_yaw) false false)
    (`|AIMoveTo` self (`KismetMathLibrary.MakeVector` _returnvalue_x _returnvalue_y _returnvalue_z) null)))

(event `LookPlayer`
  ;[1 1 1] Look to the player
  (set `self.Following Player` true)
  (bind (_direction _newtrack_0) (`Timeline|Fast Rotation` :!via `PlayFromStart`)
    (:`Update`
      (if (`self.PlayerAlive`)
        (bind (_returnvalue_roll _returnvalue_pitch _returnvalue_yaw) (`KismetMathLibrary.BreakRotator` (`KismetMathLibrary.RLerp` (`self.K2_GetActorRotation`) (`KismetMathLibrary.FindLookAtRotation` (`self.K2_GetActorLocation`) (`self.K2_GetActorLocation` (`self.As BP Third Person Character`))) _newtrack_0 true)))
        (`SceneComponent.K2_SetWorldRotation` (`self.DefaultSceneRoot`) (`KismetMathLibrary.MakeRotator` 0.0 0.0 _returnvalue_yaw) false false)
        (set `FloatingPawnMovement.MaxSpeed` 400.0 (`self.FloatingPawnMovement`))
        (`self.PursuePlayer`)))))

(fn `SendRaycast`
  (`KismetSystemLibrary.LineTraceSingle` :`Start` (`SceneComponent.K2_GetComponentLocation` (`self.RayCastEmitter`)) :`End` (`SceneComponent.K2_GetComponentLocation` (`/Game/Characters/Raccoon/Blueprints/BP_Raccoon.CameraBoom` (`self.As BP Third Person Character`))) :`TraceChannel` "TraceTypeQuery1" :`bTraceComplex` true :`DrawDebugType` "ForDuration" :`bIgnoreSelf` false)
  (`KismetSystemLibrary.K2_ClearTimer` null "SendRaycast")
  (`self.LookPlayer`))

(fn `UserConstructionScript`)