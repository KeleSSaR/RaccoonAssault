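; BP_Humano2 is a human enemy character that drives the walk state of its BPA_Humano animation Blueprint.
; A looping timer from BeginPlay polls movement velocity and sets IsWalking only when a component is positive, so purely negative movement reads as idle.
; Walking and Stoping also set the flag manually through a resettable DoOnce.
; HaciendoElKill stops the timer, clears walking, flags the kill and zeroes velocity.
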(event `self.ReceiveBeginPlay`
  (bind _asbpa_humano (cast `/Game/Characters/Enemigos/Humano/Blueprints/BPA_Humano` (`SkeletalMeshComponent.GetAnimInstance` (`self.Mesh`))))
  (set `self.As BPA Humano` _asbpa_humano)
  (bind _returnvalue (`KismetSystemLibrary.K2_SetTimerDelegate` (delegate `CuantoMeQueda`) 0.1 true))
  (`self.CuantoMeQueda`))

(event `CuantoMeQueda`
  (bind (_velocity_x _velocity_y _velocity_z) (`KismetMathLibrary.BreakVector` (`MovementComponent.Velocity` (`self.CharacterMovement`))))
  (if (or (>= _velocity_x 0.01) (>= _velocity_y 0.01) (>= _velocity_z 0.01))
    (set `/Game/Characters/Enemigos/Humano/Blueprints/BPA_Humano.isWalking` true (`self.As BPA Humano`))
    (else
      (set `/Game/Characters/Enemigos/Humano/Blueprints/BPA_Humano.isWalking` false (`self.As BPA Humano`)))))

(event `Walking`
  (`/Engine/EditorBlueprintResources/StandardMacros.DoOnce` false :!label _label
    (:`Completed`
      (set `/Game/Characters/Enemigos/Humano/Blueprints/BPA_Humano.isWalking` true (`self.As BPA Humano`)))))

(event `HaciendoElKill`
  (`KismetSystemLibrary.K2_ClearAndInvalidateTimerHandle` (stale `self.ReceiveBeginPlay` _returnvalue))
  (set `/Game/Characters/Enemigos/Humano/Blueprints/BPA_Humano.isWalking` false (`self.As BPA Humano`))
  (set `self.HaciednoElkill` true)
  (set `MovementComponent.Velocity` (0.0 0.0 0.0) (`self.CharacterMovement`)))

(event `Stoping`
  (set `/Game/Characters/Enemigos/Humano/Blueprints/BPA_Humano.isWalking` false (`self.As BPA Humano`))
  (goto _label :!via `Reset`))

(fn `UserConstructionScript`)