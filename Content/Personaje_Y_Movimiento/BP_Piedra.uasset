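; BP_Piedra is a stone actor that makes AI-detectable noise when its component hits something, then destroys itself.
; Hitting an actor tagged Enemy spawns an explosion effect and, through a DoOnce, reports noise immediately before a short delay.
; Any other hit waits longer before reporting the noise.
; Both noise reports use the stone as instigator and print a "Landed" debug message.
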(event `self.Piedra.OnComponentHit`
  (params (HitComponent :type "PrimitiveComponent Object Reference") (OtherActor :type "Actor Object Reference") (OtherComp :type "PrimitiveComponent Object Reference") (NormalImpulse :type "Vector Structure") (Hit :type "HitResult Structure (by ref)"))
  (bind _returnvalue (`self.K2_GetActorLocation`))
  (if (`self.ActorHasTag` OtherActor "Enemy")
    (`GameplayStatics.SpawnEmitterAtLocation` "/Game/StarterContent/Particles/P_Explosion.P_Explosion" (`SceneComponent.K2_GetComponentLocation` (`self.Piedra`)))
    (`/Engine/EditorBlueprintResources/StandardMacros.DoOnce` false
      (:`Completed`
        (`AISense_Hearing.ReportNoiseEvent` _returnvalue 1.0 self 3000.0)
        (`KismetSystemLibrary.PrintString` "Landed")
        (`KismetSystemLibrary.Delay` 2.0)))
    (else
      (`KismetSystemLibrary.Delay` 5.0)
      (`AISense_Hearing.ReportNoiseEvent` _returnvalue 1.0 self 3000.0)
      (`KismetSystemLibrary.PrintString` "Landed")))
  (`self.K2_DestroyActor`))

(fn `UserConstructionScript`)