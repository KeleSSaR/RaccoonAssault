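; AI controller for the human enemy that runs the BT_Humano behavior tree on BeginPlay.
; AI Perception updates go to HandleSighSense, which reacts only to sight stimuli from the player character.
; It writes the player to the TargetActor blackboard key while seen.
; When sight is lost, it clears that key and stores the stimulus position as LastKnownLocation.
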(event `self.ReceiveBeginPlay`
  (`self.RunBehaviorTree` "/Game/BluePrints/Enemigos/Humano/Blueprints/BT_Humano.BT_Humano"))

(event `self.AIPerception.OnTargetPerceptionUpdated`
  (params (Actor :type "Actor Object Reference") (Stimulus :type "AIStimulus Structure"))
  (`self.HandleSighSense` Actor Stimulus))

(fn `HandleSighSense`
  (params (Actor :type "Actor Object Reference") (Stimulus :type "AIStimulus Structure"))
  (bind (_stimulus_age _stimulus_expirationage _stimulus_strength _stimulus_stimuluslocation _stimulus_receiverlocation _stimulus_tag _stimulus_bsuccessfullysensed) (break `AIStimulus` (`local.Stimulus`)))
  (bind _returnvalue (`AIPerceptionSystem.GetSenseClassForStimulus` Stimulus))
  (if (== _returnvalue "/Script/AIModule.AISense_Sight")
    (if (== (`GameplayStatics.GetPlayerCharacter` 0) (`local.Actor`))
      (`BlackboardComponent.SetValueAsObject` (`self.Blackboard`) "TargetActor" (`KismetMathLibrary.SelectObject` (`GameplayStatics.GetPlayerCharacter` 0) null _stimulus_bsuccessfullysensed))
      (if (not _stimulus_bsuccessfullysensed)
        (`BlackboardComponent.SetValueAsVector` (`self.Blackboard`) "LastKnownLocation" _stimulus_stimuluslocation))
      (else
        (return)))
    (else
      (return))))

(fn `UserConstructionScript`)