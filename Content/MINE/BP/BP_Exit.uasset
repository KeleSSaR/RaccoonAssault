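; BP_Exit is a clickable 3D exit button that quits the game when the actor is clicked.
; BeginPlay binds cursor-over events, and two timelines lerp the static mesh's relative scale between two vectors, A and B, for a hover effect.
; The exit timeline always plays from the start with A and B swapped rather than reversing the first, so an interrupted hover snaps scale.
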(event `self.ReceiveActorOnClicked`
  (params (ButtonPressed :type "Key Structure"))
  (`KismetSystemLibrary.QuitGame` null "Quit"))

(event `self.ReceiveBeginPlay`
  (add `self.OnBeginCursorOver` (delegate `OnBeginCursorOver_Event`))
  (add `self.OnEndCursorOver` (delegate `OnEndCursorOver_Event`)))

(event `OnBeginCursorOver_Event` :!signature `self.OnBeginCursorOver`
  (params (TouchedActor :type "Actor Object Reference"))
  (bind (_direction _transicion) (`Timeline|Timeline` :!via `PlayFromStart`)
    (:`Update`
      (`SceneComponent.SetRelativeScale3D` (`self.StaticMesh`) (`KismetMathLibrary.VLerp` (`self.A`) (`self.B`) _transicion)))))

(event `OnEndCursorOver_Event` :!signature `self.OnEndCursorOver`
  (params (TouchedActor :type "Actor Object Reference"))
  (bind (_direction _transicion) (`Timeline|Timeline_0` :!via `PlayFromStart`)
    (:`Update`
      (`SceneComponent.SetRelativeScale3D` (`self.StaticMesh`) (`KismetMathLibrary.VLerp` (`self.B`) (`self.A`) _transicion)))))

(fn `UserConstructionScript`)