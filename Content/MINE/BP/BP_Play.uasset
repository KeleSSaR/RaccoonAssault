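; BP_Play is a clickable in-world Play button that hands view and control to the raccoon character.
; Clicking it blends the player camera to BP_Raccoon, enables that actor's input, and turns off the mouse cursor and click events.
; Cursor hover events bound on BeginPlay drive two timelines that lerp the mesh scale between A and B, animating it on enter and back on exit.
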(event `self.ReceiveActorOnClicked`
  (params (ButtonPressed :type "Key Structure"))
  (bind _returnvalue (`GameplayStatics.GetPlayerController` 0))
  (bind _returnvalue_2 (`GameplayStatics.GetActorOfClass` "/Game/No_Dinamico/Characters/Raccoon/BP/BP_Raccoon.BP_Raccoon_C"))
  (`PlayerController.SetViewTargetWithBlend` (`GameplayStatics.GetPlayerController` 0) _returnvalue_2 0.5 "VTBlend_Linear" 0.0 false)
  (`self.EnableInput` _returnvalue_2 null)
  (`GameplayStatics.GetActorOfClass` "/Game/No_Dinamico/Characters/Raccoon/BP/BP_Raccoon.BP_Raccoon_C")
  (set `PlayerController.bShowMouseCursor` false _returnvalue)
  (set `PlayerController.bEnableClickEvents` false _returnvalue))

(event `self.ReceiveBeginPlay`
  (add `self.OnBeginCursorOver` (delegate `OnBeginCursorOver_Event`))
  (add `self.OnEndCursorOver` (delegate `OnEndCursorOver_Event`)))

(event `OnBeginCursorOver_Event` :!signature `self.OnBeginCursorOver`
  (params (TouchedActor :type "Actor Object Reference"))
  (bind (_direction _transicion) (`Timeline|Timeline` :!via `PlayFromStart`)
    (:`Update`
      (`SceneComponent.SetRelativeScale3D` (`self.StaticMesh`) (`KismetMathLibrary.VLerp` (`self.A`) (`self.B`) _transicion)))))

(event `OnEndCursorOver_Event` :!signature `self.OnEndCursorOver`
  (params (TouchedActor :type "Actor Object Reference"))
  (bind (_direction _transicion) (`Timeline|Timeline_0` :!via `PlayFromStart`)
    (:`Update`
      (`SceneComponent.SetRelativeScale3D` (`self.StaticMesh`) (`KismetMathLibrary.VLerp` (`self.B`) (`self.A`) _transicion)))))

(fn `UserConstructionScript`)