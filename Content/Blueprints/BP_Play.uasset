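; BP_Play is a clickable 3D Play button that moves the game from its menu into gameplay.
; Clicking blends the view to the player's BP_Raccoon, enables its input and turns off cursor and click events.
; After a delay it hides itself, calls ActivarObjeto functions on cached menu and settings-camera actors, and adds food-counter and stone-cooldown widgets.
; Cursor hover events drive two timelines that lerp the mesh scale back and forth.
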(event `self.ReceiveActorOnClicked`
  (params (ButtonPressed :type "Key Structure"))
  (bind _returnvalue (`GameplayStatics.GetPlayerController` 0))
  (bind _returnvalue_2 (`GameplayStatics.GetPlayerController` 0))
  (bind _asbp_raccoon (cast `/Game/Characters/Raccoon/Blueprints/BP_Raccoon` (`GameplayStatics.GetPlayerCharacter` 0)))
  (if (`KismetSystemLibrary.IsValid` _asbp_raccoon)
    (`PlayerController.SetViewTargetWithBlend` _returnvalue _asbp_raccoon 0.5 "VTBlend_Linear" 0.0 false)
    (`self.EnableInput` _asbp_raccoon _returnvalue)
    (set `PlayerController.bShowMouseCursor` false _returnvalue_2)
    (set `PlayerController.bEnableClickEvents` false _returnvalue_2)
    (`KismetSystemLibrary.Delay` 1.0)
    (`SceneComponent.SetVisibility` (`self.SkeletalMesh`) false false)
    (`SceneComponent.SetVisibility` (`self.PLay`) false false)
    (`/Game/Characters/Raccoon/Blueprints/BP_Interface.ActivarObjeto` (`self.BP_Exit`))
    (message `/Game/Characters/Raccoon/Blueprints/BP_Interface.ActivarObjeto` (`self.BP_Ajustes`))
    (message `/Game/Characters/Raccoon/Blueprints/BP_Interface.ActivarObjeto` (`self.BP_Creditos`))
    (`/Game/Characters/Raccoon/Blueprints/BP_Interface.ActivarObjeto` (`self.BP_CamaraAjustes`))
    (`/Game/Characters/Raccoon/Blueprints/BP_Interface.ActivarObjeto` (`self.BP_caramaAjustes1`))
    (bind _returnvalue_3 (`|CreateWidget` "/Game/Blueprints/Widgets/ContadorComida/WI_ContadorComida.WI_ContadorComida_C"))
    (`UserWidget.AddToViewport` _returnvalue_3 0)
    (bind _returnvalue_4 (`|CreateWidget` "/Game/Blueprints/Widgets/CooldownPiedra/WI_CooldownPiedra.WI_CooldownPiedra_C"))
    (`UserWidget.AddToViewport` _returnvalue_4 0)))

(event `self.ReceiveBeginPlay`
  (add `self.OnBeginCursorOver` (delegate `OnBeginCursorOver_Event`))
  (`|ExecutionSequence`
    (:`then_0`
      (bind _returnvalue (`GameplayStatics.GetActorOfClass` "/Game/Blueprints/BP_Exit.BP_Exit_C"))
      (set `self.BP_Exit` _returnvalue)
      (bind _returnvalue_2 (`GameplayStatics.GetActorOfClass` "/Game/Blueprints/BP_Ajustes.BP_Ajustes_C"))
      (set `self.BP_Ajustes` _returnvalue_2)
      (bind _returnvalue_3 (`GameplayStatics.GetActorOfClass` "/Game/Blueprints/BP_Creditos.BP_Creditos_C"))
      (set `self.BP_Creditos` _returnvalue_3)
      (bind _returnvalue_4 (`GameplayStatics.GetActorOfClass` "/Game/Blueprints/BPI_camaraAjustes.BPI_camaraAjustes_C"))
      (set `self.BP_CamaraAjustes` _returnvalue_4)
      (bind _returnvalue_5 (`GameplayStatics.GetActorOfClass` "/Game/Blueprints/BPI_camaraAjustes1.BPI_camaraAjustes1_C"))
      (set `self.BP_caramaAjustes1` _returnvalue_5))
    (:`then_1`
      (add `self.OnEndCursorOver` (delegate `OnEndCursorOver_Event`)))))

(event `OnBeginCursorOver_Event` :!signature `self.OnBeginCursorOver`
  (params (TouchedActor :type "Actor Object Reference"))
  (bind (_direction _transicion) (`Timeline|Timeline` :!via `PlayFromStart`)
    (:`Update`
      (`SceneComponent.SetRelativeScale3D` (`self.SkeletalMesh`) (`KismetMathLibrary.VLerp` (`self.A`) (`self.B`) _transicion)))))

(event `OnEndCursorOver_Event` :!signature `self.OnEndCursorOver`
  (params (TouchedActor :type "Actor Object Reference"))
  (bind (_direction _transicion) (`Timeline|Timeline_0` :!via `PlayFromStart`)
    (:`Update`
      (`SceneComponent.SetRelativeScale3D` (`self.SkeletalMesh`) (`KismetMathLibrary.VLerp` (`self.B`) (`self.A`) _transicion)))))

(fn `UserConstructionScript`)