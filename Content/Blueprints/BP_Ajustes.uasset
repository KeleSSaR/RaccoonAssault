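; BP_Ajustes is a clickable actor, apparently the settings (Ajustes) object, that switches the player's view to a settings camera.
; On BeginPlay its skeletal mesh loops a controller animation.
; Clicking it finds the BPI_camaraAjustes actor, blends the view to it, and enables the mouse cursor and click events.
; Despite its name, the ActivarObjeto event hides both the skeletal and static meshes.
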(event `self.ReceiveBeginPlay`
  (`SkeletalMeshComponent.PlayAnimation` (`self.SkeletalMesh`) "/Game/No_Dinamico/Characters/Sensor/Mesh/SkeletalMesh/HUL-IO_10_COntrole.HUL-IO_10_COntrole" true))

(event `self.ReceiveActorOnClicked`
  (params (ButtonPressed :type "Key Structure"))
  (bind _returnvalue (`GameplayStatics.GetPlayerController` 0))
  (bind _returnvalue_2 (`GameplayStatics.GetActorOfClass` "/Game/Blueprints/BPI_camaraAjustes.BPI_camaraAjustes_C"))
  (`PlayerController.SetViewTargetWithBlend` _returnvalue _returnvalue_2 0.5 "VTBlend_Linear" 0.0 false)
  (set `PlayerController.bShowMouseCursor` true _returnvalue)
  (set `PlayerController.bEnableClickEvents` true _returnvalue))

(event `/Game/Characters/Raccoon/Blueprints/BP_Interface.ActivarObjeto`
  (`SceneComponent.SetVisibility` (`self.SkeletalMesh`) false false)
  (`SceneComponent.SetVisibility` (`self.StaticMesh`) false false))

(fn `UserConstructionScript`)